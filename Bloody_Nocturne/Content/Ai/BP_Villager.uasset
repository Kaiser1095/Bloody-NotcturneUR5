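; BP_Villager is an AI villager that continuously flees from the player character.
; On BeginPlay it caches the player's MC character, then starts the RunAway event.
; RunAway issues an AIMoveTo to a point 500 units directly away from the player, keeping the villager's own Z.
; Both success and failure call RunAway again, forming an endless flee loop with no distance check.
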(event `self.ReceiveBeginPlay`
  (bind _asmc (cast `/Game/ThirdPerson/Blueprints/MC` (`GameplayStatics.GetPlayerCharacter` 0)))
  (set `self.Character refrence` _asmc)
  (`self.Run Away`))

(event `Run Away`
  (bind _returnvalue (`self.K2_GetActorLocation`))
  (`|AIMoveTo` self (`KismetMathLibrary.MakeVector` (.x (+ _returnvalue (* (`KismetMathLibrary.GetForwardVector` (`KismetMathLibrary.FindLookAtRotation` _returnvalue (`self.K2_GetActorLocation` (`self.Character refrence`)))) -500.0))) (.y (+ _returnvalue (* (`KismetMathLibrary.GetForwardVector` (`KismetMathLibrary.FindLookAtRotation` _returnvalue (`self.K2_GetActorLocation` (`self.Character refrence`)))) -500.0))) (.z _returnvalue)) null
    (:`OnSuccess`
      _)
    (:`OnFail`
      _))
  (`self.Run Away`))

(fn `UserConstructionScript`)